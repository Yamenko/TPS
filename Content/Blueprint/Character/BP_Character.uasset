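; Top-down player character Blueprint that adds input-driven movement states, montages and camera setup.
; Right mouse and Left Alt switch between Aim, Walk and Run through ChangeMovementState, Space plays an ironsights or hip fire montage based on IsAim, and V plays a death montage.
; The construction script configures camera boom length, rotation and lag from variables.
; CameraShakeEvent plays a world camera shake at the camera's location.
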(event Input|KeyboardEvents|LeftAlt
  (params (Key :type Key%20Structure :default "None"))
  (:Pressed
    (Class|TPSCharacter|ChangeMovementState "Walk_state"))
  (:Released
    (Class|TPSCharacter|ChangeMovementState "Run_state")))

(event Input|KeyboardEvents|V
  (params (Key :type Key%20Structure :default "None"))
  (:Pressed
    (Animation|Montage|PlayMontage (Variables|Character|GetMesh) "/Game/Blueprint/Character/Mannequin/Animations/NewAnim/newDeath_1_Montage.newDeath_1_Montage")))

(event Input|MouseEvents|RightMouseButton
  (params (Key :type Key%20Structure :default "None"))
  (:Pressed
    (Class|TPSCharacter|ChangeMovementState "Aim_state")
    (Variables|Default|SetbIsAim true))
  (:Released
    (Class|TPSCharacter|ChangeMovementState "Run_state")
    (Variables|Default|SetbIsAim false)))

(event Input|KeyboardEvents|SpaceBar
  (params (Key :type Key%20Structure :default "None"))
  (bind _mesh (Variables|Character|GetMesh))
  (:Pressed
    (if (Variables|Default|GetbIsAim)
      (Animation|Montage|PlayMontage _mesh "/Game/Blueprint/Character/Mannequin/Animations/NewAnim/newFire_Rifle_Ironsights_Montage.newFire_Rifle_Ironsights_Montage")
      (else
        (Animation|Montage|PlayMontage _mesh "/Game/Blueprint/Character/Mannequin/Animations/NewAnim/newFire_Rifle_Hip_Montage.newFire_Rifle_Hip_Montage")))))

(fn ConstructionScript
  (bind _cameraboom (Variables|Default|GetCameraBoom))
  (Variables|/Script/Engine.SpringArmComponent|SetTargetArmLength _cameraboom (Variables|Camera|GetHeight))
  (Transformation|SetRelativeRotation _cameraboom (Variables|Camera|GetRotatorCamera) false false)
  (Variables|/Script/Engine.SpringArmComponent|SetbEnableCameraLag _cameraboom (Variables|Camera|GetFlow))
  (Variables|/Script/Engine.SpringArmComponent|SetCameraLagSpeed _cameraboom (Variables|Camera|GetCoefSmooth)))

(fn CameraShakeEvent
  (Camera|PlayWorldCameraShake "/Game/Blueprint/Game/BP_ShakeCamera.BP_ShakeCamera_C" (Transformation|GetWorldLocation (Variables|Default|GetTopDownCameraComponent)) 0.0 3e+01))