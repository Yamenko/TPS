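; BP_Door is an interactive door that swings open or closed when a BP_Character enters either of its two trigger volumes.
; Both overlaps call MoveDoor, which plays or reverses the MovingDoor timeline based on IsClose.
; The timeline drives the door's relative yaw, prints each value for debugging, and toggles IsClose on finish.
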(event OnComponentBeginOverlap(Trigger2)
  (params (OverlappedComponent :type Primitive%20Component%20Object%20Reference) (OtherActor :type Actor%20Object%20Reference) (OtherComp :type Primitive%20Component%20Object%20Reference) (OtherBodyIndex :type Integer) (bFromSweep :type Boolean) (SweepResult :type Hit%20Result%20Structure%20%28by%20ref%29))
  (Utilities|Casting|CastToBP_Character OtherActor)
  (CallFunction|MoveDoor))

(event OnComponentBeginOverlap(Trigger1)
  (params (OverlappedComponent :type Primitive%20Component%20Object%20Reference) (OtherActor :type Actor%20Object%20Reference) (OtherComp :type Primitive%20Component%20Object%20Reference) (OtherBodyIndex :type Integer) (bFromSweep :type Boolean) (SweepResult :type Hit%20Result%20Structure%20%28by%20ref%29))
  (Utilities|Casting|CastToBP_Character OtherActor)
  (CallFunction|MoveDoor))

(event Custom|MoveDoor
  (if (Variables|Default|GetIsClose)
    (bind _rotationdoor (Timeline|MovingDoor Play)
      (:Update
        (Transformation|SetRelativeRotation (Variables|Default|GetDoor) (Math|Rotator|MakeRotator 0.0 0.0 _rotationdoor) false false)
        (Development|PrintString (Utilities|String|ToString(Float) _rotationdoor)))
      (:Finished
        (Variables|Default|SetIsClose (not (Variables|Default|GetIsClose)))))
    (else
      (Timeline|MovingDoor Reverse))))

(fn ConstructionScript)